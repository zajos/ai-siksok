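; Learning Agents manager Blueprint that sets up and drives reinforcement learning training for agents.
; On BeginPlay it sets up, in order, the interactor, a policy built on that interactor and a neural network asset, and a trainer that takes both.
; Each Tick calls RunTraining on the trainer with its training, game, path and critic settings.
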(event EventBeginPlay
  (bind _bp_policy (Variables|Default|GetBP_Policy))
  (bind _bp_interactor (Variables|Default|GetBP_Interactor))
  (Utilities|FlowControl|Sequence
    (:then_0
      (Class|LearningAgentsInteractor|SetupInteractor _bp_interactor))
    (:then_1
      (Class|LearningAgentsPolicy|SetupPolicy _bp_policy _bp_interactor (Variables|Default|GetPolicySettings) "/Game/LearningAgents/NeuralNetwork.NeuralNetwork"))
    (:then_2
      (Class|LearningAgentsTrainer|SetupTrainer (Variables|Default|GetBP_Trainer) _bp_interactor _bp_policy 0 (Variables|Default|GetTrainerSettings)))))

(event EventTick
  (params (DeltaSeconds :type Float%20%28single-precision%29))
  (Class|LearningAgentsTrainer|RunTraining (Variables|Default|GetBP_Trainer) (Variables|Default|GetTrainer%20Training%20Settings) (Variables|Default|GetTrainer%20Game%20Settings) (Variables|Default|GetTrainer%20Path%20Settings) (Variables|Default|GetCritic%20Settings) true true true))

(fn ConstructionScript)